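; Shared multiplayer camera that zooms its spring arm according to how far apart two to four players are.
; After a short delay on BeginPlay, it pulls players from BP_GameMode, makes itself the controllers' view target and starts a looping UpdateCamera timer.
; The timer sets arm length to the greatest pairwise player distance.
; The result is clamped for three or four players but unclamped for two.
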(event Custom|UpdateCamera
  (switch int (Utilities|Array|Length (Variables|Default|GetPlayersReference))
    (:2
      (CallFunction|SetArmLenghtP2))
    (:3
      (CallFunction|SetArmLenghtP3))
    (:4
      (CallFunction|SetArmLenghtP4))))

(event EventBeginPlay
  (Utilities|FlowControl|Delay 2.0)
  (CallFunction|ClassSetup)
  (for _array_element (Variables|Default|GetPlayersReference)
    (Utilities|Time|SetTimerbyFunctionName 0 "UpdateCamera" 0.01 true)))

(event EventTick
  (params (DeltaSeconds :type Float%20%28single-precision%29)))

(fn ConstructionScript)

(fn ClassSetup
  (bind _asbp_game_mode (Utilities|Casting|CastToBP_GameMode (Game|GetGameMode))
    (:then
      (bind _output_get (Variables|Default|SetBP%20game%20mode _asbp_game_mode))
      (Variables|Default|SetPlayersReference (Variables|/Game/GGJ20/Blueprints/BP_GameMode.BP_GameMode_C|GetPlayers _output_get))
      (bind _outactors (Actor|GetAllActorsOfClass "/Script/Engine.PlayerController"))
      (Game|Player|SetViewTargetwithBlend _outactors self 0.0 "VTBlend_Linear" 0.0 false)
      (for (_array_element _array_index) (Variables|Default|GetPlayersReference)
        (switch int _array_index
          (:0
            (Variables|Default|SetP1 _array_element))
          (:1
            (Variables|Default|SetP2 _array_element))
          (:2
            (Variables|Default|SetP3 _array_element))
          (:3
            (Variables|Default|SetP4 _array_element)))))
    (:CastFailed
      (Development|PrintString "ERROR"))))

(fn SetArmLenghtP4
  (bind _p1 (Variables|Default|GetP1))
  (bind _p2 (Variables|Default|GetP2))
  (bind _p3 (Variables|Default|GetP3))
  (bind _p4 (Variables|Default|GetP4))
  (Development|PrintString "Hello" true true "(R=0.666667,G=0.329373,B=0.082672,A=1.000000)")
  (Variables|/Script/Engine.SpringArmComponent|SetTargetArmLength (Variables|Default|GetSpringArm) (Math|Float|Clamp(Float) (.MaxValue (Math|Float|MaxOfFloatArray (Utilities|Array|MakeArray (Transformation|GetDistanceTo _p1 _p2) (Transformation|GetDistanceTo _p1 _p3) (Transformation|GetDistanceTo _p1 _p4) (Transformation|GetDistanceTo _p2 _p3) (Transformation|GetDistanceTo _p2 _p4) (Transformation|GetDistanceTo _p3 _p4)))) (Variables|Default|GetMinValue) (Variables|Default|GetMaxValue))))

(fn SetArmLenghtP3
  (bind _p1 (Variables|Default|GetP1))
  (bind _p2 (Variables|Default|GetP2))
  (bind _p3 (Variables|Default|GetP3))
  (Variables|/Script/Engine.SpringArmComponent|SetTargetArmLength (Variables|Default|GetSpringArm) (Math|Float|Clamp(Float) (.MaxValue (Math|Float|MaxOfFloatArray (Utilities|Array|MakeArray (Transformation|GetDistanceTo _p1 _p2) (Transformation|GetDistanceTo _p1 _p3) (Transformation|GetDistanceTo _p2 _p3)))) (Variables|Default|GetMinValue) (Variables|Default|GetMaxValue))))

(fn SetArmLenghtP2
  (Variables|/Script/Engine.SpringArmComponent|SetTargetArmLength (Variables|Default|GetSpringArm) (Transformation|GetDistanceTo (Variables|Default|GetP1) (Variables|Default|GetP2))))