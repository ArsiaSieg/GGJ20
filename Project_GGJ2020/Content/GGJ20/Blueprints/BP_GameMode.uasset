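; BP_GameMode is a game mode for a GGJ20 local multiplayer game that spawns the players when play begins.
; It gathers all PlayerStart actors, then for each index below the player limit finds starts tagged with that number.
; At each match it creates a local player, spawns a BP_BouleQuiColle, has that player's controller possess it, and updates the Players list.
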(event EventBeginPlay
  (CallFunction|GetPlayerStartPoint)
  (CallFunction|SpawnPlayer))

(fn ConstructionScript)

(fn GetPlayerStartPoint
  (bind _outactors (Actor|GetAllActorsOfClass "/Script/Engine.PlayerStart"))
  (Variables|Default|SetPlayersStartArray _outactors))

(fn SpawnPlayer
  (for _index (range 0 (- (Variables|Default|GetMaxPlayerAccount) 1))
    (Variables|Default|Setindex _index)
    (for _array_element (Variables|Default|GetPlayersStartArray)
      (if (Utilities|Name|Equal(Name) (Variables|/Script/Engine.PlayerStart|GetPlayerStartTag _array_element) (Utilities|String|StringToName (Utilities|String|ToString(Integer) (Variables|Default|Getindex))))
        (Class|GameplayStatics|CreatePlayer (Variables|Default|Getindex))
        (bind _returnvalue (Game|SpawnActorfromClass "/Game/GGJ20/Blueprints/BP_BouleQuiColle.BP_BouleQuiColle_C" (Transformation|GetActorTransform _array_element) "Undefined" 0 0))
        (Pawn|Possess (Game|GetPlayerController (Variables|Default|Getindex)) _returnvalue)
        (Utilities|Array|AddUnique (Variables|Default|GetPlayers) 0)))))